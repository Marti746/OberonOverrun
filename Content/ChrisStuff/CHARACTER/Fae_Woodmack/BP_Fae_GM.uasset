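; BP_Fae_GM is a game mode that respawns the player whenever their pawn is destroyed.
; PostLogin stores and restarts the joining controller, and each restart binds the new pawn's destroyed event to restart that stored controller.
; Only one controller reference is kept, so the latest login replaces any earlier one.
; SetMusic creates and plays a fresh 2D Spaceship sound, or pauses the current one.
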(event `self.K2_PostLogin`
  (params (NewPlayer :type "PlayerController Object Reference"))
  (bind _output_get (set `self.ControllerRef` NewPlayer))
  (`self.RestartPlayer` _output_get))

(event `self.K2_OnRestartPlayer`
  (params (NewPlayer :type "Controller Object Reference"))
  (add `self.OnDestroyed` (`Controller.K2_GetPawn` NewPlayer) (delegate `PawnDied`)))

(event `PawnDied` :!signature `self.OnDestroyed`
  (params (DestroyedActor :type "Actor Object Reference"))
  (`self.RestartPlayer` (`self.ControllerRef`)))

(fn `SetMusic`
  (params (`Play?` :type Boolean))
  (if `Play?`
    (bind _returnvalue (`GameplayStatics.CreateSound2D` "/Game/FirstPerson/Music/Spaceship.Spaceship" 0.2 1.0 0.0 null))
    (bind _output_get (set `self.Music` _returnvalue))
    (`AudioComponent.Play` _output_get 0.0)
    (else
      (`AudioComponent.SetPaused` (`self.Music`) true))))

(fn `UserConstructionScript`)